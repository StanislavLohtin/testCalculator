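; Game state for planet levels that holds the available and active spell lists.
; Its construction script loads the army save game and copies in both lists, seeding three default friendly-unit summon spells when the saved available list is empty.
; If the save fails to load or cast, neither list is set, defaults included.
; The set-active-spell-and-save function is an empty stub.
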(event EventBeginPlay)

(event EventTick
  (params (DeltaSeconds :type Float%20%28single-precision%29)))

(fn ConstructionScript
  (Utilities|FlowControl|Sequence
    (:then_0
      (bind _returnvalue (SaveGame|LoadGamefromSlot (Variables|Default|GetsaveGameSlot)))
      (bind _asarmy_save_game (Utilities|Casting|CastToarmySaveGame _returnvalue))
      (Variables|Default|SetactiveSpells (Variables|/Game/Blueprints/levelClasses/armySaveGame.armySaveGame_C|GetactiveSpellList _asarmy_save_game))
      (if (== (Utilities|Array|Length (Variables|/Game/Blueprints/levelClasses/armySaveGame.armySaveGame_C|GetavailableSpellList _asarmy_save_game)) 0)
        (Utilities|Array|Add (Variables|Default|GetavailableSpells) (Utilities|Struct|MakesummonFriendlyUnitSpell "gnom2" 5 "/Game/Images/gnomIcon1.gnomIcon1" 2.0 0 "/Game/Blueprints/units/friendly/friendlyUnit1.friendlyUnit1_C"))
        (Utilities|Array|Add (Variables|Default|GetavailableSpells) (Utilities|Struct|MakesummonFriendlyUnitSpell "strelok" 10 "/Game/Images/sold1.sold1" 3.0 0 "/Game/Blueprints/units/friendly/friendlyUnit2.friendlyUnit2_C"))
        (Utilities|Array|Add (Variables|Default|GetavailableSpells) (Utilities|Struct|MakesummonFriendlyUnitSpell "geroi avtomatchik" 0 "/Game/Images/sold2.sold2" 2e+01 10 "/Game/Blueprints/units/friendly/friendlyUnit3.friendlyUnit3_C"))
        (Development|PrintString "setting default avail spells")
        (else
          (Variables|Default|SetavailableSpells (Variables|/Game/Blueprints/levelClasses/armySaveGame.armySaveGame_C|GetavailableSpellList _asarmy_save_game)))))))

(fn SetActiveSpellandSave)