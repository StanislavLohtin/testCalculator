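; Base pawn for friendly units in a lane-based 2D game that walk along -Y and auto-attack hostiles.
; Tick polls a range box, sized from Autoattack.Range at construction, to toggle walking and a looping cooldown timer that fires projectiles or damages everything in range.
; With nothing in range, it picks the closest visible hostile, biased toward its own lane, and shifts one lane toward it by delayed teleport.
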(event Custom|autoattackingTicker
  ;[1 1 1] start Autoattacking
  (Variables|Default|SetattackOnCooldown false)
  (if (Variables|Default|GetisAutoattacking)
    (CallFunction|DoAutoattack)
    (else
      (CallFunction|StopAutoattacking))))

(event EventBeginPlay
  (|CallParentFunction))

(event Collision|EventActorBeginOverlap
  (params (OtherActor :type Actor%20Object%20Reference))
  (|CallParentFunction OtherActor) ; This node is disabled and will not be called.\nDrag off pins to build functionality.
)

(event EventTick
  (params (DeltaSeconds :type Float%20%28single-precision%29))
  (bind _currentlane (Variables|Default|GetcurrentLane))
  (|CallParentFunction DeltaSeconds)
  (Utilities|FlowControl|Sequence
    (:then_0
      (if (Variables|Default|GetisChangingLane)
        (if (not (.isRanged (Utilities|Struct|BreakattackType (Variables|Default|Getautoattack))))
          (Pawn|Input|AddMovementInput "0.000000,-1.000000,0.000000" (/ (Math|Conversions|ToFloat(Integer) (Variables|Default|GetmovementSpeed)) 1e+03) false))
        (elif (and (Variables|Default|GetisWalking) (not (Variables|Default|GetisAutoattacking)))
          (Pawn|Input|AddMovementInput "0.000000,-1.000000,0.000000" (/ (Math|Conversions|ToFloat(Integer) (Variables|Default|GetmovementSpeed)) 2e+02) false))))
    (:then_1
      (if (Variables|Default|GetisAutoattacking)
        ;[1 1 1] stopAutoAttacking
        (bind _hostiles (CallFunction|GetAllOverlappingHostiles))
        (if (== (Utilities|Array|Length _hostiles) 0)
          (Variables|Default|SetisAutoattacking false)
          (Variables|Default|SetisWalking true))
        (else
          (bind _hostiles_2 (CallFunction|GetAllOverlappingHostiles))
          (if (> (Utilities|Array|Length _hostiles_2) 0)
            ;[1 1 1] start Autoattacking
            (Variables|Default|SetisWalking false)
            (Variables|Default|SetisAutoattacking true)
            (if (not (Variables|Default|GetattackOnCooldown))
              (bind _returnvalue (Utilities|Time|SetTimerbyEvent (delegate Custom|autoattackingTicker) (.cooldown (Utilities|Struct|BreakattackType (Variables|Default|Getautoattack))) true 0.0 0.05))
              (Variables|Default|SetattackingTimer _returnvalue)
              (CallFunction|DoAutoattack))
            (else
              ;[1 1 1] selectEnemyAndMaybeChangeLine
              (bind _hostiles_3 (CallFunction|GetAllHostilesinVision))
              (if (> (Utilities|Array|Length _hostiles_3) 0)
                (bind (_closesthostile _isonalllanes) (CallFunction|GetClosestHostileinVision _hostiles_3))
                (if (not _isonalllanes)
                  (if (not (== (Variables|/Game/Blueprints/parentClasses/BP_destructablePawn.BP_destructablePawn_C|GetcurrentLane _closesthostile) _currentlane))
                    (Utilities|MoveUporDown (> (Variables|/Game/Blueprints/parentClasses/BP_destructablePawn.BP_destructablePawn_C|GetcurrentLane _closesthostile) _currentlane))))))))))))

(fn ConstructionScript
  (|CallParentFunction)
  (Utilities|FlowControl|Sequence
    (:then_0
      (Variables|/Script/Engine.FloatingPawnMovement|SetMaxSpeed (Variables|Default|GetpawnMovement) (Math|Conversions|ToFloat(Integer) (Variables|Default|GetmovementSpeed))))
    (:then_1
      (CallFunction|UpdateAttackRangeBoxSize))))

(fn GetAllOverlappingHostiles
  (bind _rangecollisionchecker (Variables|Default|GetrangeCollisionChecker))
  (bind _result (LocalVariables|Getresult))
  (for _array_element (Collision|GetOverlappingActors _rangecollisionchecker "/Game/Blueprints/parentClasses/BP_destructableHostilePawn.BP_destructableHostilePawn_C" :!class /Script/Engine.PrimitiveComponent)
    (bind _asbp_destructable_hostile_pawn (Utilities|Casting|CastToBP_destructableHostilePawn _array_element))
    (if (Utilities|Array|ContainsItem (Class|PrimitiveComponent|GetOverlappingComponents _rangecollisionchecker) (Variables|/Game/Blueprints/parentClasses/BP_destructablePawn.BP_destructablePawn_C|GetcollisionBox _asbp_destructable_hostile_pawn))
      (Utilities|Array|Add _result _asbp_destructable_hostile_pawn)))
  (return _result))

(fn GetAllHostilesinVision
  (bind _visionrange (Variables|Default|GetvisionRange))
  (bind _result (LocalVariables|Getresult))
  (for _array_element (Collision|GetOverlappingActors _visionrange "/Game/Blueprints/parentClasses/BP_destructableHostilePawn.BP_destructableHostilePawn_C" :!class /Script/Engine.PrimitiveComponent)
    (bind _asbp_destructable_hostile_pawn (Utilities|Casting|CastToBP_destructableHostilePawn _array_element))
    (if (Utilities|Array|ContainsItem (Class|PrimitiveComponent|GetOverlappingComponents _visionrange) (Variables|/Game/Blueprints/parentClasses/BP_destructablePawn.BP_destructablePawn_C|GetcollisionBox _asbp_destructable_hostile_pawn))
      (Utilities|Array|Add _result _asbp_destructable_hostile_pawn)))
  (return _result))

(fn HasHostileonSameLane
  (params (Array :type Array%20of%20BP%20Destructable%20Hostile%20Pawn%20Object%20References))
  (bind _array_element (Utilities|Array|ForEachLoopwithBreak Array)
    (:LoopBody
      (if (== (Variables|/Game/Blueprints/parentClasses/BP_destructablePawn.BP_destructablePawn_C|GetcurrentLane _array_element) (Variables|Default|GetcurrentLane))
        (return true)))
    (:Completed
      (return false))))

(fn GetDifferenceinMillis
  (params (dateTime :type Date%20Time%20Structure))
  (bind _returnvalue (Math|DateTime|Now))
  (bind _returnvalue_2 (- _returnvalue dateTime))
  (bind (_days _hours _minutes _seconds _milliseconds) (Math|Timespan|BreakTimespan _returnvalue_2))
  (return (* (+ (* (+ (* _hours 60) _minutes) 60) _seconds) _milliseconds)))

(fn GetClosestHostileinVision
  (params (visibleHostiles :type Array%20of%20BP%20Destructable%20Hostile%20Pawn%20Object%20References))
  (bind _self self)
  (bind _returnvalue (Transformation|GetActorLocation _self))
  (for _array_element visibleHostiles
    ;[1 1 1] ifVisibleHostileIsAFence
    (Utilities|Casting|CastTohostile2DBaseUnit _array_element
      (:then
        (if (== (Variables|/Game/Blueprints/parentClasses/BP_destructablePawn.BP_destructablePawn_C|GetcurrentLane _array_element) (Variables|Default|GetcurrentLane _self))
          (if (< (- (Class|KismetMathLibrary|GetPointDistancetoSegment (Transformation|GetActorLocation _array_element) _returnvalue _returnvalue) (LocalVariables|GetmovingToAnotherLineThreshold)) (LocalVariables|GetclosestDistance)) :!label _label
            (LocalVariables|SetclosestDistance (Class|KismetMathLibrary|GetPointDistancetoSegment (Transformation|GetActorLocation _array_element) _returnvalue _returnvalue) :!label _label_2)
            (LocalVariables|Setresult _array_element))
          (elif (< (Class|KismetMathLibrary|GetPointDistancetoSegment (Transformation|GetActorLocation _array_element) _returnvalue _returnvalue) (LocalVariables|GetclosestDistance))
            (goto _label_2))))
      (:CastFailed
        (goto _label))))
  (Utilities|Casting|CastTohostile2DBaseUnit (LocalVariables|Getresult)
    (:then
      (return (LocalVariables|Getresult) false))
    (:CastFailed
      (return (LocalVariables|Getresult) false))))

(fn DoAutoattack
  (bind _autoattack (Variables|Default|Getautoattack))
  (bind (_mindamage _maxdamage _critchance _critdamage _cooldown _range _sound _isranged _hitsonlyfirsttarget _projectilespeed _projectileclass) (Utilities|Struct|BreakattackType _autoattack))
  (Variables|Default|SetattackOnCooldown true)
  (if _isranged
    (if _hitsonlyfirsttarget
      (Game|SpawnActorfromClass _projectileclass (Math|Transform|MakeTransform (Transformation|GetWorldLocation (Variables|Default|GetprojectileOrigin)) "0.000000,180.000000, 0") "Undefined" 0 (Variables|Default|Getautoattack) true self 0)
      (Audio|PlaySound2D _sound 0.3 1.0 0.0 0 0)
      (return))
    (elif (not _hitsonlyfirsttarget)
      (Utilities|DamageAllPawnsinRange
        (:Completed
          (return))))))

(fn UpdateAttackRangeBoxSize
  (bind _rangecollisionchecker (Variables|Default|GetrangeCollisionChecker))
  (bind _autoattack (Variables|Default|Getautoattack))
  (bind _range (Utilities|Struct|BreakattackType _autoattack))
  (bind _returnvalue (/ _range 2))
  (Components|Box|SetBoxExtent _rangecollisionchecker (Math|Vector|MakeVector 5e+01 (Math|Conversions|ToFloat(Integer) _returnvalue) 1e+02) true)
  (Transformation|SetRelativeLocation _rangecollisionchecker (Math|Vector|MakeVector 0.0 (Math|Conversions|ToFloat(Integer) (* (- _returnvalue 10) -1)) 1e+02) false false))

(fn StopAutoattacking
  (Utilities|Time|ClearandInvalidateTimerbyHandle (Variables|Default|GetattackingTimer))
  (return))