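; Parent pawn for damageable 2D sprite units, with a health bar widget that is linked to the pawn on BeginPlay.
; DamagePawn rolls random damage with a crit multiplier, subtracts health, plays a sound and spawns floating damage text projected to screen space with random jitter.
; At zero health it destroys itself, and hostile subclasses add one blood to the fight game state.
; A helper offsets the sprite in fixed grid steps.
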(event EventBeginPlay
  (bind _aswb_health_bar (Utilities|Casting|CastToWB_healthBar (UserInterface|GetUserWidgetObject (Variables|Default|Gethealthbar))))
  (Variables|/Game/Blueprints/UI/WB_healthBar.WB_healthBar_C|SetdestructablePawn _aswb_health_bar self))

(event Collision|EventActorBeginOverlap
  (params (OtherActor :type Actor%20Object%20Reference)))

(event EventTick
  (params (DeltaSeconds :type Float%20%28single-precision%29)))

(fn ConstructionScript)

(fn DamagePawn
  (params (damagingAttack :type Attack%20Type%20Structure))
  (bind (_mindamage _maxdamage _critchance _critdamage) (Utilities|Struct|BreakattackType damagingAttack))
  (Utilities|FlowControl|Sequence
    (:then_0
      (bind _output_get (LocalVariables|SetrandomDamage (Math|Random|RandomIntegerinRange _mindamage _maxdamage)))
      (bind _output_get_2 (LocalVariables|SetisCritical (> _critchance (Math|Random|RandomFloatinRange 0.0 1e+02))))
      (if _output_get_2
        (LocalVariables|SetrandomDamage (Math|Float|Truncate (* _output_get _critdamage)))))
    (:then_1
      (bind _output_get_3 (Variables|Default|SetcurrentHealth (- (Variables|Default|GetcurrentHealth) (LocalVariables|GetrandomDamage))))
      (Audio|PlaySound2D "/Game/sounds/missMelee2.missMelee2" 1.0 1.0 0.0 0 0)
      (CallFunction|SpawnDamageText (LocalVariables|GetrandomDamage) (LocalVariables|GetisCritical))
      (if (<= _output_get_3 0)
        (Actor|DestroyActor)
        (Utilities|Casting|CastToBP_destructableHostilePawn self)
        (bind _asfight_level_game_state (Utilities|Casting|CastTofightLevelGameState (Game|GetGameState)))
        (Variables|/Game/Blueprints/levelClasses/fightLevelGameState.fightLevelGameState_C|SetcurrentBlood _asfight_level_game_state (+ (Variables|/Game/Blueprints/levelClasses/fightLevelGameState.fightLevelGameState_C|GetcurrentBlood _asfight_level_game_state) 1))))))

(fn SetSpriteLocation
  (params (spriteXLocation :type Integer) (spriteYLocation :type Integer))
  (bind _papersprite (Variables|Default|GetPaperSprite))
  (bind _relativelocation (Variables|/Script/Engine.SceneComponent|GetRelativeLocation _papersprite))
  (bind (_x _y _z) (Math|Vector|BreakVector _relativelocation))
  (Transformation|SetRelativeLocation _papersprite (Math|Vector|MakeVector (+ (Math|Conversions|ToFloat(Integer) (* spriteXLocation 20)) _x) (+ (Math|Conversions|ToFloat(Integer) (* spriteYLocation 15)) _y) _z) false false)
  (return))

(fn SpawnDamageText
  (params (damageAmount :type Integer) (isDamageCritical :type Boolean))
  (bind _returnvalue (UserInterface|CreateWidget "/Game/Blueprints/UI/WB_floatingDamageText.WB_floatingDamageText_C" 0 damageAmount isDamageCritical (.ScreenPosition (Class|GameplayStatics|ProjectWorldtoScreen (Game|GetPlayerController 0) (+ (Transformation|GetWorldLocation (Variables|Default|Gethealthbar)) (Variables|Default|GetdamageTextLocation) (Math|Vector|MakeVector 0.0 (Math|Conversions|ToFloat(Integer) (* (Math|Random|RandomIntegerinRange -1 1) 20)) 0.0)) false))))
  (UserInterface|Viewport|AddtoViewport _returnvalue 0)
  (return))