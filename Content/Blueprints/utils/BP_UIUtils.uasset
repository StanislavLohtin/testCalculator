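; BP_UIUtils is a set of UI helpers that restyle buttons by an enabled flag, such as when resources are insufficient.
; SetButtonBGIfNotEnoughResource rebuilds the style from the button's Normal brush for normal, hovered and pressed states, tinting it translucent dark blue when disabled.
; SetButtonPositionIfEnabled nudges the button down with a render transform when enabled and resets the transform otherwise.
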(fn SetButtonBGifNotEnoughResource
  (params (button :type Button%20Object%20Reference) (isEnabled :type Boolean))
  (bind _widgetstyle (Variables|/Script/UMG.Button|GetWidgetStyle button))
  (bind _normal (Utilities|Struct|BreakButtonStyle _widgetstyle))
  (if isEnabled
    (bind _structout (Utilities|Struct|SetmembersinSlateBrush _normal "(SpecifiedColor=(R=1.000000,G=1.000000,B=1.000000,A=1.000000),ColorUseRule=UseColor_Specified)"))
    (Class|Button|SetStyle button (Utilities|Struct|MakeButtonStyle _structout _structout _structout))
    (else
      (bind _structout_2 (Utilities|Struct|SetmembersinSlateBrush _normal (Utilities|Struct|MakeSlateColor "(R=0.028592,G=0.046694,B=0.322917,A=0.800000)")))
      (Class|Button|SetStyle button (Utilities|Struct|MakeButtonStyle _structout_2 _structout_2 _structout_2)))))

(fn SetButtonPositionifEnabled
  (params (isEnabled :type Boolean) (button :type Button%20Object%20Reference))
  (if isEnabled
    (Class|Widget|SetRenderTransform button (Utilities|Struct|MakeWidgetTransform "(X=0.000000,Y=5.000000)"))
    (else
      (Class|Widget|SetRenderTransform button (Utilities|Struct|MakeWidgetTransform "(X=0.000000,Y=0.000000)"))))
  (return))