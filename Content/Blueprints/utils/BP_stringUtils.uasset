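; BP_stringUtils is a string utility Blueprint that formats numeric values, named as times, into decimal text with a suffix.
; The float function splits the stringified value at the decimal point and cuts the fraction to the requested precision.
; The integer function joins separate seconds and milliseconds the same way, without zero-padding the milliseconds.
; Both truncate by substring rather than rounding.
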(fn FloattoStringwithSuffix
  (params (timeFloat :type Float%20%28single-precision%29) (precision :type Integer) (suffix :type String))
  (bind _returnvalue (Utilities|String|ToString(Float) timeFloat))
  (bind _returnvalue_2 (Utilities|String|ParseIntoArray _returnvalue "."))
  (return (Utilities|String|Append (Utilities|Array|Get(acopy) _returnvalue_2) "." (Utilities|String|GetSubstring (Utilities|Array|Get(acopy) _returnvalue_2 1) 0 precision) suffix)))

(fn IntegerstoStringwithSuffix
  (params (seconds :type Integer) (milliseconds :type Integer) (precision :type Integer) (suffix :type String))
  (return (Utilities|String|Append (Utilities|String|ToString(Integer) seconds) "." (Utilities|String|GetSubstring (Utilities|String|ToString(Integer) milliseconds) 0 precision) suffix)))