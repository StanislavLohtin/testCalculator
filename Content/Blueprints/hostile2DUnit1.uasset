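; Hostile 2D unit that walks along +Y and auto-attacks friendly destructible pawns within its attack range.
; The construction script sets health and sizes and offsets a box range checker from Attack1's range.
; Tick toggles between walking and attacking based on friendlies whose CollisionBox overlaps that box.
; Entering combat hits all of them immediately, then a looping cooldown timer repeats the hit and clears itself once attacking stops.
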(event Custom|autoattackingTicker
  (if (Variables|Default|GetisAutoattacking)
    (Utilities|DamageAllPawnsinRange)
    (else
      (Utilities|Time|ClearandInvalidateTimerbyHandle (stale EventTick _returnvalue)))))

(event EventBeginPlay
  (|CallParentFunction))

(event Collision|EventActorBeginOverlap
  (params (OtherActor :type Actor%20Object%20Reference))
  (|CallParentFunction OtherActor) ; This node is disabled and will not be called.\nDrag off pins to build functionality.
)

(event EventTick
  (params (DeltaSeconds :type Float%20%28single-precision%29))
  (|CallParentFunction DeltaSeconds)
  (Utilities|FlowControl|Sequence
    (:then_0
      (if (Variables|Default|GetisWalking)
        (Pawn|Input|AddMovementInput "0.000000,1.000000,0.000000" (/ (Math|Conversions|ToFloat(Integer) (Variables|Default|GetmovementSpeed)) 2e+02) false)))
    (:then_1
      (if (Variables|Default|GetisAutoattacking)
        (bind _hostiles (CallFunction|GetAllOverlappingFriendlies))
        (if (== (Utilities|Array|Length _hostiles) 0)
          (Variables|Default|SetisAutoattacking false)
          (Variables|Default|SetisWalking true))
        (else
          (bind _hostiles_2 (CallFunction|GetAllOverlappingFriendlies))
          (if (> (Utilities|Array|Length _hostiles_2) 0)
            (Variables|Default|SetisAutoattacking true)
            (Variables|Default|SetisWalking false)
            (bind _returnvalue (Utilities|Time|SetTimerbyEvent (delegate Custom|autoattackingTicker) (.cooldown (Utilities|Struct|BreakattackType (Variables|Default|Getattack1))) true 0.0 0.3))
            (Utilities|DamageAllPawnsinRange)))))))

(fn ConstructionScript
  (bind _rangecollisionchecker (Variables|Default|GetrangeCollisionChecker))
  (bind _attack1 (Variables|Default|Getattack1))
  (bind _range (Utilities|Struct|BreakattackType _attack1))
  (bind _returnvalue (/ _range 2))
  (|CallParentFunction)
  (Variables|Default|SetcurrentHealth 70)
  (Variables|Default|SetmaxHealth 70)
  (Variables|Default|SetdamageTextLocation "0,20.000000,150.000000")
  (Components|Box|SetBoxExtent _rangecollisionchecker (Math|Vector|MakeVector 5e+01 (Math|Conversions|ToFloat(Integer) _returnvalue) 1e+02) true)
  (Transformation|SetRelativeLocation _rangecollisionchecker (Math|Vector|MakeVector 0.0 (Math|Conversions|ToFloat(Integer) (- _returnvalue 10)) 1e+02) false false))

(fn GetAllOverlappingFriendlies
  (bind _rangecollisionchecker (Variables|Default|GetrangeCollisionChecker))
  (bind _result (LocalVariables|Getresult))
  (for _array_element (Collision|GetOverlappingActors _rangecollisionchecker "/Game/Blueprints/parentClasses/BP_destructableFriendlyPawn.BP_destructableFriendlyPawn_C" :!class /Script/Engine.PrimitiveComponent)
    (bind _asbp_destructable_friendly_pawn (Utilities|Casting|CastToBP_destructableFriendlyPawn _array_element))
    (if (Utilities|Array|ContainsItem (Class|PrimitiveComponent|GetOverlappingComponents _rangecollisionchecker) (Variables|/Game/Blueprints/parentClasses/BP_destructablePawn.BP_destructablePawn_C|GetcollisionBox _asbp_destructable_friendly_pawn))
      (Utilities|Array|Add _result _asbp_destructable_friendly_pawn)))
  (return _result))