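; Base projectile actor that carries an AttackType, which sets its movement speed at construction and is passed to the damage call on impact.
; When HitsOnlyHostiles is set, overlapping a destructible hostile pawn's CollisionBox damages that pawn and destroys the projectile.
; Under the same flag, leaving the friendly shooter's RangeCollisionChecker destroys it after a brief delay, capping travel at the unit's range.
; A fixed lifetime timer started at BeginPlay also destroys it.
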(event OnComponentBeginOverlap(collisionCapsule)
  (params (OverlappedComponent :type Primitive%20Component%20Object%20Reference) (OtherActor :type Actor%20Object%20Reference) (OtherComp :type Primitive%20Component%20Object%20Reference) (OtherBodyIndex :type Integer) (bFromSweep :type Boolean) (SweepResult :type Hit%20Result%20Structure%20%28by%20ref%29))
  (if (Variables|Default|GethitsOnlyHostiles)
    (bind _asbp_destructable_hostile_pawn (Utilities|Casting|CastToBP_destructableHostilePawn OtherActor))
    (if (== OtherComp (Variables|/Game/Blueprints/parentClasses/BP_destructablePawn.BP_destructablePawn_C|GetcollisionBox _asbp_destructable_hostile_pawn))
      (Default|DamagePawn _asbp_destructable_hostile_pawn (Variables|Default|GetattackType))
      (Actor|DestroyActor))))

(event OnComponentEndOverlap(collisionCapsule)
  (params (OverlappedComponent :type Primitive%20Component%20Object%20Reference) (OtherActor :type Actor%20Object%20Reference) (OtherComp :type Primitive%20Component%20Object%20Reference) (OtherBodyIndex :type Integer))
  (if (and (Variables|Default|GethitsOnlyHostiles) (== (Variables|Default|GetshooterPawn) OtherActor))
    (bind _asfriendly_2dbase_unit (Utilities|Casting|CastTofriendly2DBaseUnit OtherActor))
    (if (== OtherComp (Variables|/Game/Blueprints/friendly2DBaseUnit.friendly2DBaseUnit_C|GetrangeCollisionChecker _asfriendly_2dbase_unit))
      (Utilities|FlowControl|Delay 0.05)
      (Actor|DestroyActor))))

(event EventBeginPlay
  (Utilities|FlowControl|Delay 8.0)
  (Actor|DestroyActor))

(event Collision|EventActorBeginOverlap
  (params (OtherActor :type Actor%20Object%20Reference)))

(event EventTick
  (params (DeltaSeconds :type Float%20%28single-precision%29)))

(fn ConstructionScript
  (bind _projectilemovement (Variables|Default|GetprojectileMovement))
  (bind _attacktype (Variables|Default|GetattackType))
  (bind _projectilespeed (Utilities|Struct|BreakattackType _attacktype))
  (bind _returnvalue (Math|Conversions|ToFloat(Integer) _projectilespeed))
  (Variables|/Script/Engine.ProjectileMovementComponent|SetMaxSpeed _projectilemovement _returnvalue)
  (Variables|/Script/Engine.ProjectileMovementComponent|SetInitialSpeed _projectilemovement _returnvalue))