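; Shuttle actor for the planet view that flies along a given path when FlyToPlanet is called.
; A timeline, with play rate set from the path's travel duration, drives an alpha curve from start to end of the path's spline.
; Each update moves and rotates the actor to the world-space spline location and rotation at that distance.
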(event Custom|FlyToPlanet
  (params (shuttlePath :type Shuttle%20Path%20on%20Planet%20Object%20Reference))
  (bind _pathspline (Variables|/Game/Blueprints/planetView/shuttlePathOnPlanet.shuttlePathOnPlanet_C|GetPathSpline shuttlePath))
  (Components|Timeline|SetPlayRate (Variables|Default|GetshuttleMover) (/ 1.0 (Variables|/Game/Blueprints/planetView/shuttlePathOnPlanet.shuttlePathOnPlanet_C|GettravelDuration shuttlePath)))
  (bind _alphacurve (Timeline|shuttleMover Play)
    (:Update
      (bind _output_get (Variables|Default|SetalphaCurve _alphacurve))
      (Transformation|SetActorLocationAndRotation (Spline|GetLocationatDistanceAlongSpline _pathspline (Math|Float|Lerp 0.0 (Spline|GetSplineLength _pathspline) _output_get) "World") (Spline|GetRotationatDistanceAlongSpline _pathspline (Math|Float|Lerp 0.0 (Spline|GetSplineLength _pathspline) _output_get) "World")))))

(event EventBeginPlay)

(event Collision|EventActorBeginOverlap
  (params (OtherActor :type Actor%20Object%20Reference)))

(event EventTick
  (params (DeltaSeconds :type Float%20%28single-precision%29)))

(fn ConstructionScript)