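; Clickable level marker in the planet view, labeled with its GameLevel number and tinted red when locked.
; Hovering an unlocked marker enlarges its cube and shows a widget, both reverted when the cursor leaves.
; Clicking calls LevelClickedEvent if unlocked, otherwise prints a locked message.
; Direct level loading by file name remains in the graph but never runs.
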(event OnBeginCursorOver(Cube)
  (params (TouchedComponent :type Primitive%20Component%20Object%20Reference))
  (bind _cube (Variables|Default|GetCube))
  (if (not (.isLocked (Utilities|Struct|BreakgameLevel (Variables|Default|GetgameLevel))))
    (Variables|Default|SetisHovered true)
    (Transformation|SetRelativeScale3D _cube (* (Transformation|GetWorldScale _cube) "1.200000,1.200000,1.200000"))
    (Rendering|SetVisibility (Variables|Default|GetWidget) true true)))

(event OnClicked(Cube)
  (params (TouchedComponent :type Primitive%20Component%20Object%20Reference) (ButtonPressed :type Key%20Structure :default "None"))
  (if (.isLocked (Utilities|Struct|BreakgameLevel (Variables|Default|GetgameLevel)))
    (Development|PrintString "level is LOCKED!!")
    (else
      (Default|CallLevelClickedEvent))))

(event OnEndCursorOver(Cube)
  (params (TouchedComponent :type Primitive%20Component%20Object%20Reference))
  (bind _cube (Variables|Default|GetCube))
  (if (Variables|Default|GetisHovered)
    (Variables|Default|SetisHovered false)
    (Transformation|SetRelativeScale3D _cube (/ (Transformation|GetWorldScale _cube) "1.200000,1.200000,1.200000"))
    (Rendering|SetVisibility (Variables|Default|GetWidget) false true)))

(event EventBeginPlay
  (bind _gamelevel (Variables|Default|GetgameLevel))
  (bind _levelnumber (Variables|Default|GetlevelNumber))
  (bind (_number _islocked) (Utilities|Struct|BreakgameLevel _gamelevel))
  (Rendering|Components|TextRender|SetText _levelnumber (Utilities|Text|ToText(String) (Utilities|String|Append "Level " (Utilities|String|ToString(Integer) _number))))
  (if _islocked
    (Rendering|Components|TextRender|SetTextRenderColor _levelnumber (Math|Color|MakeColor 40 40 255 1))))

(event Collision|EventActorBeginOverlap
  (params (OtherActor :type Actor%20Object%20Reference)))

(event EventTick
  (params (DeltaSeconds :type Float%20%28single-precision%29)))

(fn ConstructionScript)